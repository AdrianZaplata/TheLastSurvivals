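; BP_TimerBoost is a pickup that adds time to the match timer when the player's TopDownCharacter overlaps its static mesh.
; On overlap it plays a pickup sound, destroys itself and adds its AddTime value to TimeSec on the TopDownGameMode, found via GetActorOfClass.
; A single rollover step carries seconds past 59 into TimeMin.
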(event `self.ReceiveBeginPlay`)

(event `self.StaticMesh.OnComponentBeginOverlap`
  (params (OverlappedComponent :type "PrimitiveComponent Object Reference") (OtherActor :type "Actor Object Reference") (OtherComp :type "PrimitiveComponent Object Reference") (OtherBodyIndex :type Integer) (bFromSweep :type Boolean) (SweepResult :type "HitResult Structure (by ref)"))
  (cast `/Game/TopDownBP/Blueprints/TopDownCharacter` OtherActor)
  (`GameplayStatics.PlaySound2D` "/Game/TheLastSurvivors/Music/Time_pick_up.Time_pick_up" 1.0 1.0 0.0 null null)
  (`self.K2_DestroyActor`)
  (bind _returnvalue (`GameplayStatics.GetActorOfClass` "/Game/TopDownBP/Blueprints/TopDownGameMode.TopDownGameMode_C"))
  (bind _timesec (`/Game/TopDownBP/Blueprints/TopDownGameMode.TimeSec` _returnvalue))
  (set `/Game/TopDownBP/Blueprints/TopDownGameMode.TimeSec` (+ (`self.AddTime`) _timesec) _returnvalue)
  (if (> _timesec 59)
    (set `/Game/TopDownBP/Blueprints/TopDownGameMode.TimeMin` (+ (`/Game/TopDownBP/Blueprints/TopDownGameMode.TimeMin` _returnvalue) 1) _returnvalue)
    (set `/Game/TopDownBP/Blueprints/TopDownGameMode.TimeSec` (- _timesec 60) _returnvalue)))

(fn `UserConstructionScript`)